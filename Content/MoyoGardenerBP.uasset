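; Gardener neighbor NPC that greets the player and receives items through interaction.
; Its Interactable event either sends a greeting when the player controller's inventory is empty or passes the first item's ID to the interacting Character's SendItem.
; The greeting and receive events advance NeighborState and show stage 2 text through the game mode, with receipt also removing the item from RemainingItems.
; Death calls the parent and prints a debug string.
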(event Custom|ChefInteract
  (params (Controller :type Player%20Controller%20Object%20Reference) (Character :type Moyo%20Character%20Object%20Reference))
  (bind _asmoyo_player_controller (Utilities|Casting|CastToMoyoPlayerController Controller))
  (if (== (Utilities|Array|Length (Variables|/Script/Moyo.MoyoPlayerController|GetInventory _asmoyo_player_controller)) 0)
    (Class|MoyoGuy|SendGreeting)
    (else
      (Class|MoyoGuy|SendItem Character (.ItemID (Utilities|Struct|BreakInventoryItem (Utilities|Array|Get(acopy) (Variables|/Script/Moyo.MoyoPlayerController|GetInventory _asmoyo_player_controller))))))))

(event EventDoDeath
  (|CallParentFunction)
  (Development|PrintString "ohno"))

(event EventBeginPlay
  (EventDispatchers|BindEventtoOnInteractEvent (Variables|Default|GetInteractable) (delegate Custom|ChefInteract)))

(event EventDoRecieve
  (params (itemID :type Name :default "None"))
  (Utilities|Array|RemoveItem (Variables|Default|GetRemainingItems) itemID)
  (Variables|Default|SetNeighborState "NewEnumerator2")
  (Default|Text (stale EventDoGreeting _asmoyo_game_mode_bp) 2 1))

(event EventDoGreeting
  (Variables|Default|SetNeighborState "NewEnumerator1")
  (bind _asmoyo_game_mode_bp (Utilities|Casting|CastToMoyoGameModeBP (Game|GetGameMode)))
  (Default|Text _asmoyo_game_mode_bp 2))

(fn ConstructionScript)