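; Game mode that manages the game's intro, play and finish states and serves dialog text.
; BeginPlay loads title and fail screens as hidden level instances; SetState toggles their visibility on state changes and opens the Islands level for play.
; Text stores a stage and line, then lazily spawns and activates a DialogDataActor, which GetDialog queries while active and CloseDialog deactivates.
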(event EventBeginPlay
  (Utilities|FlowControl|Sequence
    (:then_0
      (bind _returnvalue (Class|LevelStreamingDynamic|LoadLevelInstance "/Game/TitleStream" "0, 0, 0" "0, 0, 0"))
      (bind _output_get (Variables|Default|Settitlestream _returnvalue))
      (Variables|/Script/Engine.LevelStreaming|SetbShouldBeVisible _output_get false))
    (:then_1
      (bind _returnvalue_2 (Class|LevelStreamingDynamic|LoadLevelInstance "/Game/FailStream" "0, 0, 0" "0, 0, 0"))
      (bind _output_get_2 (Variables|Default|Setfailstream _returnvalue_2))
      (Variables|/Script/Engine.LevelStreaming|SetbShouldBeVisible _output_get_2 false))))

(event EventTick
  (params (DeltaSeconds :type Float%20%28single-precision%29)))

(fn ConstructionScript)

(fn SetState
  (params (InState :type EMoyoGameState%20Enum :default "NONE"))
  (if (Utilities|Enum|NotEqual(Enum) InState (Variables|Default|GetLastState))
    (Utilities|FlowControl|Sequence
      (:then_0
        (switch Utilities|FlowControl|Switch|SwitchonEMoyoGameState (Variables|Default|GetLastState)
          (:INTRO
            (Variables|/Script/Engine.LevelStreaming|SetbShouldBeVisible (Variables|Default|Gettitlestream) false))
          (:FINISH
            (Variables|/Script/Engine.LevelStreaming|SetbShouldBeVisible (Variables|Default|Getfailstream) false))))
      (:then_1
        (bind _output_get (Variables|Default|SetLastState InState))
        (switch Utilities|FlowControl|Switch|SwitchonEMoyoGameState _output_get
          (:INTRO
            (Variables|/Script/Engine.LevelStreaming|SetbShouldBeVisible (Variables|Default|Gettitlestream) true))
          (:PLAY
            (Game|OpenLevel(byName) "Islands"))
          (:FINISH
            (Variables|/Script/Engine.LevelStreaming|SetbShouldBeVisible (Variables|Default|Getfailstream) true)))))))

(fn GetDialog
  (bind _dialogactor (Variables|Default|Getdialogactor)
    (:then
      (if (Variables|/Game/DialogDataActor.DialogDataActor_C|GetIsActive _dialogactor)
        (bind _word (Default|GetDialog (Variables|Default|Getdialogactor) (Variables|Default|Getdialogstage) (Variables|Default|Getdialogline)))
        (return _word)
        (else
          (return ""))))
    (:else
      (return ""))))

(fn OpenDialog
  (Utilities|FlowControl|Sequence
    (:then_0
      (Variables|Default|Getdialogactor
        (:then)
        (:else
          (bind _returnvalue (Game|SpawnActorfromClass "/Game/DialogDataActor.DialogDataActor_C" (Math|Transform|MakeTransform "0, 0, 0") "Undefined" 0 0))
          (Variables|Default|Setdialogactor _returnvalue))))
    (:then_1
      (Variables|/Game/DialogDataActor.DialogDataActor_C|SetIsActive (Variables|Default|Getdialogactor) true))))

(fn CloseDialog
  (Variables|/Game/DialogDataActor.DialogDataActor_C|SetIsActive (Variables|Default|Getdialogactor) false))

(fn Text
  (params (stage :type Integer) (line :type Integer))
  (Utilities|FlowControl|Sequence
    (:then_0
      (Variables|Default|Setdialogstage stage))
    (:then_1
      (Variables|Default|Setdialogline line))
    (:then_2
      (CallFunction|OpenDialog))))